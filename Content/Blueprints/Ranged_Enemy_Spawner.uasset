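; Ranged enemy spawner actor that repeatedly spawns BP_EnemyArcher at its Sphere component's location and rotation.
; Tick increments the TimeToSpawn counter by one per frame, then spawns and resets it on reaching a hard-coded threshold, so the interval depends on frame rate.
; Each archer's AIControllerClass is set to AI_Enemy after SpawnActor returns, and spawning has no count limit.
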(event `self.ReceiveTick`
  (params (DeltaSeconds :type "Float (single-precision)"))
  (bind _timetospawn (`self.TimeToSpawn`))
  (bind _sphere (`self.Sphere`))
  (if (== 540.0 _timetospawn)
    (set `self.TimeToSpawn` 0.0)
    (bind _returnvalue (`|SpawnActorFromClass` "/Game/TopDown/Blueprints/Characters/BP_EnemyArcher.BP_EnemyArcher_C" (`KismetMathLibrary.MakeTransform` (`SceneComponent.K2_GetComponentLocation` _sphere) (`SceneComponent.K2_GetComponentRotation` _sphere)) "Undefined" "OverrideRootScale" null null))
    (set `Pawn.AIControllerClass` "/Game/Blueprints/AI_Enemy.AI_Enemy_C" _returnvalue)
    (else
      (set `self.TimeToSpawn` (+ _timetospawn 1.0)))))

(fn `UserConstructionScript`)